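; BP_Blade is a grabbable VR weapon that works as a grappling hook, pulling the player toward a traced point.
; Grabbing enables input and adds a right or left grapple mapping context by holding hand; dropping disables it.
; Right shoot line-traces from TestChainSpawner, attaches Cable to a spawned hook actor and starts a looping timer offsetting the pawn.
; Canceling either hand hides Cable and clears the timer; left shoot otherwise only prints debug text.
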(event OnGrabbed(GrabComponent)
  ;[0 0 0] When the Weapon  is grabbed, enable input and add the Weapon Input Mapping Context. Disable and remove when the Wepon  is dropped.
  (Input|EnableInput (Game|GetPlayerController 0))
  (Input|AddMappingContext (PlayerController|LocalPlayerSubsystems|GetEnhancedInputLocalPlayerSubsystem (Game|GetPlayerController 0)) (select (Utilities|Enum|Equal(Enum) (Default|GetHeldbyHand (Variables|Default|GetGrabComponent)) "Right") "/Game/VRTemplate/Input/IMC_GrappleR.IMC_GrappleR" "/Game/VRTemplate/Input/IMC_GrappleL.IMC_GrappleL") 1 "(bIgnoreAllPressedKeysUntilRelease=True,bForceImmediately=False)"))

(event OnDropped(GrabComponent)
  ;[0 0 0] When the Weapon  is grabbed, enable input and add the Weapon Input Mapping Context. Disable and remove when the Wepon  is dropped.
  (Input|DisableInput (Game|GetPlayerController 0))
  (Input|RemoveMappingContext (PlayerController|LocalPlayerSubsystems|GetEnhancedInputLocalPlayerSubsystem (Game|GetPlayerController 0)) 0 "(bIgnoreAllPressedKeysUntilRelease=True,bForceImmediately=False)"))

(event Custom|PlayerPull
  (bind _returnvalue (Utilities|Time|SetTimerbyEvent (delegate Custom|PlayerPull) 0.01 true))
  (Variables|Default|SetPulling _returnvalue)
  (Transformation|AddActorWorldOffset (Variables|Default|GetPlayerVR%20Ref) (* (- (Variables|Default|GetAttachPoint) (Transformation|GetActorLocation)) (Variables|Default|GetPullingForce))))

(event Input|EnhancedActionEvents|EnhancedInputActionIA_Shoot_Right
  (params (ActionValue :type Boolean) (ElapsedSeconds :type Float%20%28double-precision%29) (TriggeredSeconds :type Float%20%28double-precision%29) (InputAction :type Input%20Action%20Object%20Reference :default "/Game/VRTemplate/Input/Actions/IA_Shoot_Right.IA_Shoot_Right"))
  (bind _testchainspawner (Variables|Default|GetTestChainSpawner))
  (bind _returnvalue (Transformation|GetWorldLocation _testchainspawner))
  (:Triggered
    (Development|PrintString "Hello"))
  (:Started
    (bind (_outhit _returnvalue_2) (Collision|LineTraceByChannel _returnvalue (+ _returnvalue (* (Math|Vector|GetForwardVector (Transformation|GetWorldRotation _testchainspawner)) (Variables|Default|GetPullingDistance))) "TraceTypeQuery1" false 0 "None"))
    (if _returnvalue_2
      (Development|SetHiddeninGame (Variables|Default|GetCable) false false)
      ;[1 1 1] Check where it hit
      (bind _output_get (Variables|Default|SetAttachPoint (.Location (Collision|BreakHitResult _outhit))))
      (bind _returnvalue_3 (Game|SpawnActorfromClass "/Game/FER_DEV/Blueprints/BP_HookActorTest.BP_HookActorTest_C" (Math|Transform|MakeTransform _output_get "0, 0, 0" "1.000000,1.000000,1.000000") "Undefined" "MultiplyWithRoot" 0 0))
      (Class|CableComponent|SetAttachEndto (Variables|Default|GetCable) _returnvalue_3 "None" "None")
      (CallFunction|PlayerPull)))
  (:Canceled
    (Development|SetHiddeninGame (Variables|Default|GetCable) true false)
    ;[1 1 1] Forces ¨Pulling¨ event to stop
    (Utilities|Time|ClearandInvalidateTimerbyHandle (Variables|Default|GetPulling))))

(event Input|EnhancedActionEvents|EnhancedInputActionIA_Shoot_Left
  (params (ActionValue :type Boolean) (ElapsedSeconds :type Float%20%28double-precision%29) (TriggeredSeconds :type Float%20%28double-precision%29) (InputAction :type Input%20Action%20Object%20Reference :default "/Game/VRTemplate/Input/Actions/IA_Shoot_Left.IA_Shoot_Left"))
  (:Triggered
    (Development|PrintString "Hello"))
  (:Canceled
    (Development|SetHiddeninGame (Variables|Default|GetCable) true false)
    ;[1 1 1] Forces ¨Pulling¨ event to stop
    (Utilities|Time|ClearandInvalidateTimerbyHandle (Variables|Default|GetPulling))))

(event EventBeginPlay
  (bind _asvrpawn (Utilities|Casting|CastToVRPawn (Game|Player|GetPlayerPawn 0)))
  (bind _output_get (Variables|Default|SetPlayerVR%20Ref _asvrpawn))
  (Variables|Default|SetRightHandRef (Variables|/Game/VRTemplate/Blueprints/VRPawn.VRPawn_C|GetHandRight _output_get))
  (Variables|Default|SetLeftHandRef (Variables|/Game/VRTemplate/Blueprints/VRPawn.VRPawn_C|GetHandLeft _output_get))
  (Utilities|FlowControl|Sequence))

(event Collision|EventActorBeginOverlap
  (params (OtherActor :type Actor%20Object%20Reference)))

(event EventTick
  (params (DeltaSeconds :type Float%20%28single-precision%29)))

(fn ConstructionScript)