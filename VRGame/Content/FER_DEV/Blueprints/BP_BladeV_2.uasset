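; BP_BladeV_2 is a grappling projectile that, once it hits something, pulls the owning BP_GrapplingPlayer toward itself.
; A sphere hit stops the projectile, disables gravity on the player's capsule and starts grappling.
; While grappling, Tick adds PullForce to the capsule along the direction from the motion controller to the blade, with debug prints.
; Destroying the blade restores gravity and ends the grapple.
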(event OnComponentHit(Sphere)
  (params (HitComponent :type Primitive%20Component%20Object%20Reference) (OtherActor :type Actor%20Object%20Reference) (OtherComp :type Primitive%20Component%20Object%20Reference) (NormalImpulse :type Vector :default "0, 0, 0") (Hit :type Hit%20Result%20Structure%20%28by%20ref%29))
  (Components|Movement|StopMovementImmediately (Variables|Default|GetProjectileMovement))
  (Physics|SetEnableGravity (Variables|/Script/Engine.Character|GetCapsuleComponent (Variables|Default|GetVRCharRef)) false)
  (Development|PrintString "Hello")
  (Variables|Default|SetGrappling true))

(event EventTick
  (params (DeltaSeconds :type Float%20%28single-precision%29))
  (Development|PrintString (Utilities|String|ToString(Vector) (Transformation|GetWorldLocation (Variables|Default|GetMotionController))) true true "(R=0.879366,G=1.000000,B=0.000000,A=1.000000)")
  (if (Variables|Default|GetGrappling)
    (Physics|AddForce (Variables|/Script/Engine.Character|GetCapsuleComponent (Variables|Default|GetVRCharRef)) (* (Math|Vector|GetForwardVector (Math|Rotator|FindLookatRotation (Transformation|GetWorldLocation (Variables|Default|GetMotionController)) (Transformation|GetActorLocation))) (Variables|Default|GetPullForce)) "None" false)
    (Development|PrintString "APPLY?" true true "(R=1.000000,G=0.135948,B=0.000000,A=1.000000)")))

(event EventBeginPlay
  (Actor|Tick|SetActorTickEnabled true))

(event EventDestroyed
  (Physics|SetEnableGravity (Variables|/Script/Engine.Character|GetCapsuleComponent (Variables|Default|GetVRCharRef)) true)
  (Variables|Default|SetGrappling false))

(fn ConstructionScript
  (bind _asbp_grappling_player (Utilities|Casting|CastToBP_GrapplingPlayer (Components|GetOwner)))
  (Variables|Default|SetVRCharRef _asbp_grappling_player))