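; VR player Blueprint that gives each hand a grappling blade, held out for as long as that hand's trigger is pressed.
; BeginPlay adds the default and hands Enhanced Input mapping contexts.
; Each trigger press spawns a scaled-down BP_BladeV_2 at its motion controller and passes it the player and controller references; release destroys it.
; The left and right grapple mapping contexts are unwired, and Tick has no effect.
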(event Input|EnhancedActionEvents|EnhancedInputActionIA_Shoot_Left
  (params (ActionValue :type Boolean) (ElapsedSeconds :type Float%20%28double-precision%29) (TriggeredSeconds :type Float%20%28double-precision%29) (InputAction :type Input%20Action%20Object%20Reference :default "/Game/VRTemplate/Input/Actions/IA_Shoot_Left.IA_Shoot_Left")))

(event Input|EnhancedActionEvents|EnhancedInputActionIA_Shoot_Right
  (params (ActionValue :type Boolean) (ElapsedSeconds :type Float%20%28double-precision%29) (TriggeredSeconds :type Float%20%28double-precision%29) (InputAction :type Input%20Action%20Object%20Reference :default "/Game/VRTemplate/Input/Actions/IA_Shoot_Right.IA_Shoot_Right")))

(event EventBeginPlay
  (bind _returnvalue (Game|GetPlayerController 0))
  (bind _returnvalue_2 (PlayerController|LocalPlayerSubsystems|GetEnhancedInputLocalPlayerSubsystem _returnvalue))
  (Input|AddMappingContext _returnvalue_2 "/Game/VRTemplate/Input/IMC_Default.IMC_Default" 0 "(bIgnoreAllPressedKeysUntilRelease=True,bForceImmediately=False)")
  (Input|AddMappingContext _returnvalue_2 "/Game/VRTemplate/Input/IMC_Hands.IMC_Hands" 0 "(bIgnoreAllPressedKeysUntilRelease=True,bForceImmediately=False)"))

(event EventTick
  (params (DeltaSeconds :type Float%20%28single-precision%29))
  (Utilities|FlowControl|DoOnce false))

(event Input|ActionEvents|InputActionTriggerRight
  (params (Key :type Key%20Structure :default "None"))
  (bind _motioncontrollerright (Variables|Default|GetMotionControllerRight))
  (bind _returnvalue (Transformation|GetWorldTransform _motioncontrollerright))
  (:Pressed
    (bind _returnvalue_2 (Game|SpawnActorfromClass "/Game/FER_DEV/Blueprints/BP_BladeV_2.BP_BladeV_2_C" (Math|Transform|MakeTransform (.location _returnvalue) (.rotation _returnvalue) "0.100000,0.100000,0.100000") "AlwaysSpawn" "MultiplyWithRoot" 0 0))
    (bind _output_get (Variables|Default|SetGrapplingBladeRight _returnvalue_2))
    (Variables|/Game/FER_DEV/Blueprints/BP_BladeV_2.BP_BladeV_2_C|SetVRCharRef _output_get self)
    (Variables|/Game/FER_DEV/Blueprints/BP_BladeV_2.BP_BladeV_2_C|SetMotionController _output_get (Variables|Default|GetMotionControllerRight)))
  (:Released
    (Actor|DestroyActor (Variables|Default|GetGrapplingBladeRight))))

(event Input|ActionEvents|InputActionTriggerLeft
  (params (Key :type Key%20Structure :default "None"))
  (bind _motioncontrollerleft (Variables|Default|GetMotionControllerLeft))
  (bind _returnvalue (Transformation|GetWorldTransform _motioncontrollerleft))
  (:Pressed
    (bind _returnvalue_2 (Game|SpawnActorfromClass "/Game/FER_DEV/Blueprints/BP_BladeV_2.BP_BladeV_2_C" (Math|Transform|MakeTransform (.location _returnvalue) (.rotation _returnvalue) "0.100000,0.100000,0.100000") "AlwaysSpawn" "MultiplyWithRoot" 0 0))
    (bind _output_get (Variables|Default|SetGrapplingBladeLeft _returnvalue_2))
    (Variables|/Game/FER_DEV/Blueprints/BP_BladeV_2.BP_BladeV_2_C|SetVRCharRef _output_get self)
    (Variables|/Game/FER_DEV/Blueprints/BP_BladeV_2.BP_BladeV_2_C|SetMotionController _output_get (Variables|Default|GetMotionControllerLeft)))
  (:Released
    (Actor|DestroyActor (Variables|Default|GetGrapplingBladeLeft))))

(fn ConstructionScript)